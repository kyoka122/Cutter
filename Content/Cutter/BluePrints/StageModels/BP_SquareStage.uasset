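; BP_SquareStage is a stage model Blueprint that describes the bounds of a square stage.
; On BeginPlay it sets fixed minimum and maximum 2D corners, symmetric around a center at the origin.
; Getter functions expose the corners, center and radius, though the radius variable is never assigned in these graphs.
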(event EventBeginPlay
  (Variables|Default|SetEdgeMin "(X=-750.000000,Y=-750.000000)")
  (Variables|Default|SetEdgeMax "(X=750.000000,Y=750.000000)")
  (Variables|Default|SetCenterPos "0, 0, 0"))

(fn ConstructionScript)

(fn GetEdgeMin
  (return (Variables|Default|GetEdgeMin)))

(fn GetEdgeMax
  (return (Variables|Default|GetEdgeMax)))

(fn GetCenterPos
  (return (Variables|Default|GetCenterPos)))

(fn GetRadius
  (return (Variables|Default|GetStageRadius)))