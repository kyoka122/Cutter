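; BP_CutterBlowe is a configurable Niagara tornado effect actor with a spline and an invisible collider exposed through GetStaticMesh.
; ApplyChanges pushes scale, color, shape, ribbon, sprite and smoke settings into NSTornado, from both the construction script and BeginPlay.
; MoveAlongPath and ChasePlayer implement spline-following and player-chasing steps.
; The MovementMode switch meant to drive movement by looping timers is disconnected and never runs.
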(event EventBeginPlay
  (CallFunction|ApplyChanges))

(fn ConstructionScript
  (CallFunction|ApplyChanges)
  (Spline|SetClosedLoop (Variables|Default|GetSpline) (Variables|General|GetLoop%20Spline) true))

(fn ApplyChanges
  (bind _ns_tornado (Variables|Default|GetNS_Tornado))
  (bind _ns_tornado_2 (Variables|Default|GetNS_Tornado))
  (bind _scale (Variables|General|GetScale))
  (bind _ns_tornado_3 (Variables|Default|GetNS_Tornado))
  (bind _scale_2 (Variables|General|GetScale))
  (bind _ns_tornado_4 (Variables|Default|GetNS_Tornado))
  (bind _returnvalue (Math|Conversions|ToVector2D(Vector) _scale_2))
  ;[0.3005 0 0 0.121] Boolean Parameters
  (Effects|Components|ParticleSystem|SetBoolParameter _ns_tornado_2 "Enable Sprite" (Variables|Sprite|GetSprite))
  (Effects|Components|ParticleSystem|SetBoolParameter _ns_tornado_2 "Enable Smoke" (Variables|GroundSmoke|GetGround%20Smoke))
  (Utilities|FlowControl|Sequence
    (:then_1
      ;[0.02843 0.402 0.000911 0.354] Float Parameters
      (Niagara|SetNiagaraVariable(Float) _ns_tornado_3 "Lifetime" (* _scale 1e+01))
      (Niagara|SetNiagaraVariable(Float) _ns_tornado_3 "Spawn Rate Multiplier" _scale)
      (Niagara|SetNiagaraVariable(Float) _ns_tornado_3 "Ribbon Width" (Variables|Ribbon|GetRibbon%20Width))
      (Niagara|SetNiagaraVariable(Float) _ns_tornado_3 "Sprite Height" (/ 8e+02 (Variables|General|GetScale))))
    (:then_2
      ;[0 0.0999 0.5906 0.183] Vector 2D Parameters
      (Niagara|SetNiagaraVariable(LinearColor) _ns_tornado_4 "Color" (Variables|General|GetColor))
      (Class|NiagaraComponent|SetVariableVec2 _ns_tornado_4 "SmokeCurveScale" (Math|Vector2D|MakeVector2D 1.0 (* 2.5 _scale_2)))
      (Class|NiagaraComponent|SetVariableVec2 _ns_tornado_4 "Scale Curve" _returnvalue)
      (Class|NiagaraComponent|SetVariableVec2 _ns_tornado_4 "Sprite Scale" _returnvalue))
    (:then_3
      ;[0.9911 0.5841 0.01681 0.229] Vector Parameters
      (Niagara|SetNiagaraVariable(Vector3) _ns_tornado "Shape Curve X" (Variables|General|GetShape%20Curve%20X))
      (Niagara|SetNiagaraVariable(Vector3) _ns_tornado "Shape Curve Y" (Variables|General|GetShape%20Curve%20Y))
      (Transformation|SetWorldScale3D _ns_tornado (Math|Conversions|ToVector(Float) (Variables|General|GetScale)))
      (Niagara|SetNiagaraVariable(Vector3) _ns_tornado "SpawnRate" (Math|Vector|MakeVector (Variables|Ribbon|GetRibbon%20Spawn%20Rate) (Variables|Sprite|GetSprite%20Spawn%20Rate) (Variables|GroundSmoke|GetSmoke%20Spawn%20Rate))))))

(fn MoveAlongPath
  (Variables|Private|SetDistance%20Along%20Spline (+ (* 0.01 (Variables|General|GetMovement%20Speed)) (Variables|Private|GetDistance%20Along%20Spline)))
  (Transformation|SetRelativeLocation (Variables|Default|GetNS_Tornado) (Spline|GetLocationatDistanceAlongSpline (Variables|Default|GetSpline) (Variables|Private|GetDistance%20Along%20Spline) "Local") false false)
  (if (Variables|General|GetLoop%20Spline)
    (if (> (Variables|Private|GetDistance%20Along%20Spline) (Spline|GetSplineLength (Variables|Default|GetSpline)))
      (Variables|Private|SetDistance%20Along%20Spline 0.0))))

(fn ChasePlayer
  (Transformation|SetActorLocation (+ (Transformation|GetActorLocation self) (* (Math|Vector|Normalize (- (Transformation|GetActorLocation (Game|GetPlayerCharacter 0)) (Transformation|GetActorLocation self))) (Variables|General|GetMovement%20Speed))) false false))

(fn GetStaticMesh
  (return (Variables|Default|GetCollider_InVisible)))